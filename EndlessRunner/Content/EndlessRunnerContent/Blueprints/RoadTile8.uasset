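; Endless runner road tile that fills itself with obstacles and pickups and extends the track.
; On BeginPlay, three lanes roll in sequence for trunk, log, honey or magnet, re-rolling per check; an empty lane skips those after it.
; Player overlap with Box has the game mode spawn a tile, adds multiplied points and raises walk speed within limits.
; Tick destroys the tile after a delay once the camera passes SpawnPoint.
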(event `self.ReceiveBeginPlay`
  (`self.SpawnObstacles`))

(event `self.ReceiveTick`
  (params (DeltaSeconds :type "Float (single-precision)"))
  (bind _returnvalue_x (`KismetMathLibrary.BreakVector` (`SceneComponent.K2_GetComponentLocation` (`self.SpawnPoint`))))
  (bind _asthird_person_character (cast `/Game/ThirdPersonBP/Blueprints/ThirdPersonCharacter` (`GameplayStatics.GetPlayerCharacter` 0)))
  (bind _returnvalue_x_2 (`KismetMathLibrary.BreakVector` (`SceneComponent.K2_GetComponentLocation` (`/Game/ThirdPersonBP/Blueprints/ThirdPersonCharacter.FollowCamera` _asthird_person_character))))
  (if (>= (- _returnvalue_x_2 _returnvalue_x) 500.0)
    (`KismetSystemLibrary.Delay` 2.0)
    (`self.K2_DestroyActor`)))

(event `self.Box.OnComponentBeginOverlap`
  (params (OverlappedComponent :type "PrimitiveComponent Object Reference") (OtherActor :type "Actor Object Reference") (OtherComp :type "PrimitiveComponent Object Reference") (OtherBodyIndex :type Integer) (bFromSweep :type Boolean) (SweepResult :type "HitResult Structure (by ref)"))
  (cast `/Game/ThirdPersonBP/Blueprints/ThirdPersonCharacter` OtherActor)
  (bind _asthird_person_game_mode (cast `/Game/ThirdPersonBP/Blueprints/ThirdPersonGameMode` (`GameplayStatics.GetGameMode`)))
  (`/Game/ThirdPersonBP/Blueprints/ThirdPersonGameMode.SpawnTile` _asthird_person_game_mode)
  (bind _asthird_person_game_mode_2 (cast `/Game/ThirdPersonBP/Blueprints/ThirdPersonGameMode` (`GameplayStatics.GetGameMode`)))
  (set `/Game/ThirdPersonBP/Blueprints/ThirdPersonGameMode.CurrentPoints` (+ (`/Game/ThirdPersonBP/Blueprints/ThirdPersonGameMode.CurrentPoints` _asthird_person_game_mode_2) (* 1 (`/Game/ThirdPersonBP/Blueprints/ThirdPersonGameMode.PointsMultiplier` _asthird_person_game_mode_2))) _asthird_person_game_mode_2)
  (bind _asthird_person_character (cast `/Game/ThirdPersonBP/Blueprints/ThirdPersonCharacter` (`GameplayStatics.GetPlayerCharacter` 0)))
  (bind _charactermovement (`Character.CharacterMovement` _asthird_person_character))
  (set `CharacterMovementComponent.MaxWalkSpeed` (`KismetMathLibrary.FClamp` (* (`CharacterMovementComponent.MaxWalkSpeed` _charactermovement) 1.006) 600.0 2400.0) _charactermovement))

(fn `SpawnObstacles`
  (bind _returnvalue (`KismetMathLibrary.RandomFloatInRange` 0.0 2.0))
  (bind _returnvalue_2 (`KismetMathLibrary.RandomFloatInRange` 0.0 2.0))
  (bind _returnvalue_3 (`KismetMathLibrary.RandomFloatInRange` 0.0 2.0))
  (bind _returnvalue_4 (`SceneComponent.K2_GetComponentToWorld` (`self.Lane0`)))
  (bind _returnvalue_5 (`SceneComponent.K2_GetComponentToWorld` (`self.Lane2`)))
  (bind _returnvalue_6 (`SceneComponent.K2_GetComponentToWorld` (`self.Lane1`)))
  ;[1 1 1] Lane 0
  (if (`KismetMathLibrary.InRange_FloatFloat` _returnvalue 0.0 0.4)
    (`|SpawnActorFromClass` "/Game/EndlessRunnerContent/Blueprints/Obstacle_Trunk.Obstacle_Trunk_C" _returnvalue_4 "Undefined" "OverrideRootScale" null null)
    ;[1 1 1] Lane 1
    (if (`KismetMathLibrary.InRange_FloatFloat` _returnvalue_2 0.0 0.4) :!label _label
      (`|SpawnActorFromClass` "/Game/EndlessRunnerContent/Blueprints/Obstacle_Trunk.Obstacle_Trunk_C" _returnvalue_6 "Undefined" "OverrideRootScale" null null)
      ;[1 1 1] Lane 2
      (if (`KismetMathLibrary.InRange_FloatFloat` _returnvalue_3 0.0 0.4) :!label _label_2
        (`|SpawnActorFromClass` "/Game/EndlessRunnerContent/Blueprints/Obstacle_Trunk.Obstacle_Trunk_C" _returnvalue_5 "Undefined" "OverrideRootScale" null null)
        (elif (`KismetMathLibrary.InRange_FloatFloat` _returnvalue_3 0.4 0.5)
          (`|SpawnActorFromClass` "/Game/EndlessRunnerContent/Blueprints/Obstacle_TreeLog.Obstacle_TreeLog_C" _returnvalue_5 "Undefined" "OverrideRootScale" null null)
          (elif (`KismetMathLibrary.InRange_FloatFloat` _returnvalue_3 0.5 0.95)
            (`|SpawnActorFromClass` "/Game/EndlessRunnerContent/Blueprints/Honey_Pickup.Honey_Pickup_C" _returnvalue_5 "Undefined" "OverrideRootScale" null null)
            (elif (`KismetMathLibrary.InRange_FloatFloat` _returnvalue_3 0.95)
              (`|SpawnActorFromClass` "/Game/EndlessRunnerContent/Blueprints/Magnet_Pickup.Magnet_Pickup_C" _returnvalue_5 "Undefined" "OverrideRootScale" null null)))))
      (elif (`KismetMathLibrary.InRange_FloatFloat` _returnvalue_2 0.4 0.5)
        (`|SpawnActorFromClass` "/Game/EndlessRunnerContent/Blueprints/Obstacle_TreeLog.Obstacle_TreeLog_C" _returnvalue_6 "Undefined" "OverrideRootScale" null null)
        (goto _label_2)
        (elif (`KismetMathLibrary.InRange_FloatFloat` _returnvalue_2 0.5 0.95)
          (`|SpawnActorFromClass` "/Game/EndlessRunnerContent/Blueprints/Honey_Pickup.Honey_Pickup_C" _returnvalue_6 "Undefined" "OverrideRootScale" null null)
          (goto _label_2)
          (elif (`KismetMathLibrary.InRange_FloatFloat` _returnvalue_2 0.95)
            (`|SpawnActorFromClass` "/Game/EndlessRunnerContent/Blueprints/Magnet_Pickup.Magnet_Pickup_C" _returnvalue_6 "Undefined" "OverrideRootScale" null null)
            (goto _label_2)))))
    (elif (`KismetMathLibrary.InRange_FloatFloat` _returnvalue 0.4 0.5)
      (`|SpawnActorFromClass` "/Game/EndlessRunnerContent/Blueprints/Obstacle_TreeLog.Obstacle_TreeLog_C" _returnvalue_4 "Undefined" "OverrideRootScale" null null)
      (goto _label)
      (elif (`KismetMathLibrary.InRange_FloatFloat` _returnvalue 0.5 0.95)
        (`|SpawnActorFromClass` "/Game/EndlessRunnerContent/Blueprints/Honey_Pickup.Honey_Pickup_C" _returnvalue_4 "Undefined" "OverrideRootScale" null null)
        (goto _label)
        (elif (`KismetMathLibrary.InRange_FloatFloat` _returnvalue 0.95)
          (`|SpawnActorFromClass` "/Game/EndlessRunnerContent/Blueprints/Magnet_Pickup.Magnet_Pickup_C" _returnvalue_4 "Undefined" "OverrideRootScale" null null)
          (goto _label))))))

(fn `UserConstructionScript`)